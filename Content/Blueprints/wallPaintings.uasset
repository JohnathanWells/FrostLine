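; Wall painting actor that shows how many fishermen are left through five X components, presumably marks crossing out painted figures.
; UpdateWall switches on the FishermenLeft count, revealing X5 at four left and one more X per step down to all five at zero.
; Any other count hides all five; the numbered cases only reveal marks and never hide them.
; The event graph and construction script are empty.
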(fn `UpdateWall`
  (params (`Fishermen Left` :type Integer))
  (bind _x4 (`self.x4`))
  (bind _x5 (`self.x5`))
  (switch `int` `Fishermen Left`
    (:`Default`
      (`SceneComponent.SetVisibility` _x4 false false)
      (`SceneComponent.SetVisibility` _x5 false false)
      (`SceneComponent.SetVisibility` (`self.x3`) false false)
      (`SceneComponent.SetVisibility` (`self.x1`) false false)
      (`SceneComponent.SetVisibility` (`self.x2`) false false))
    (:`0`
      (`SceneComponent.SetVisibility` _x5 true false)
      (`SceneComponent.SetVisibility` _x4 true false)
      (`SceneComponent.SetVisibility` (`self.x3`) true false)
      (`SceneComponent.SetVisibility` (`self.x2`) true false)
      (`SceneComponent.SetVisibility` (`self.x1`) true false))
    (:`1`
      (`SceneComponent.SetVisibility` (`self.x2`) true false)
      (`SceneComponent.SetVisibility` (`self.x3`) true false)
      (`SceneComponent.SetVisibility` _x4 true false)
      (`SceneComponent.SetVisibility` _x5 true false))
    (:`2`
      (`SceneComponent.SetVisibility` (`self.x3`) true false)
      (`SceneComponent.SetVisibility` _x4 true false)
      (`SceneComponent.SetVisibility` _x5 true false))
    (:`3`
      (`SceneComponent.SetVisibility` _x4 true false)
      (`SceneComponent.SetVisibility` _x5 true false))
    (:`4`
      (`SceneComponent.SetVisibility` _x5 true false))))

(fn `UserConstructionScript`)