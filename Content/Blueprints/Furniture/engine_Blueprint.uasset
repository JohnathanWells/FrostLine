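; Engine furniture Blueprint that serves as the win objective, tracking three pieces handed in to it.
; CheckLights takes a Pieces array and a HUD, clears each held piece, switches its matching light to the EngineOn material and records it in IntroducedKeys.
; Once all three keys are recorded, it tells the HUD to show the win message.
; The event graph and construction script are empty.
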(fn `CheckLights`
  (params (Pieces :type "Array of Boolean (by ref)") (HUD :type "/Game/Blueprints/HUD Object Reference"))
  (bind _introduced_keys (`self.Introduced Keys`))
  (for (_array_element _array_index) Pieces
    (if _array_element
      (`KismetArrayLibrary.Array_Set` Pieces _array_index false)
      (switch `int` _array_index
        (:`0`
          (`PrimitiveComponent.SetMaterial` (`self.Light 1`) 0 "/Game/Assets/Materials/engineOn.engineOn"))
        (:`1`
          (`PrimitiveComponent.SetMaterial` (`self.Light 2`) 0 "/Game/Assets/Materials/engineOn.engineOn"))
        (:`2`
          (`PrimitiveComponent.SetMaterial` (`self.Light 3`) 0 "/Game/Assets/Materials/engineOn.engineOn")))
      (`KismetArrayLibrary.Array_Set` _introduced_keys _array_index true)))
  (if (and (`KismetArrayLibrary.Array_Get` _introduced_keys) (`KismetArrayLibrary.Array_Get` _introduced_keys 1) (`KismetArrayLibrary.Array_Get` _introduced_keys 2))
    (`/Game/Blueprints/HUD.Show Win Message` HUD))
  (return))

(fn `UserConstructionScript`)