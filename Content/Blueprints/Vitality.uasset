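; Vitality blueprint that tracks clamped integer Health, Heat and Energy values, each with a normalized float for UI.
; Modify functions clamp their value and update the matching float.
; Tick regenerates Health below maximum after a countdown that restarts whenever Health drops below its last saved value.
; Regeneration accumulates in a float seeded by a resettable DoOnce, then floors into Health directly without updating HealthF.
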(event `self.ReceiveTick`
  (params (DeltaSeconds :type "Float (single-precision)"))
  (`self.Regenerate Health` DeltaSeconds))

(fn `Get Energy UI`
  (returns (NewParam :type "Float (double-precision)"))
  (return (/ (`KismetMathLibrary.Conv_IntToDouble` (`self.Energy`)) 1000.0)))

(fn `Get Health UI`
  (returns (NewParam :type "Float (double-precision)"))
  (return (/ (`KismetMathLibrary.Conv_IntToDouble` (`self.Health`)) 100.0)))

(fn `Get Heat UI`
  (returns (NewParam :type "Float (double-precision)"))
  (return (/ (`KismetMathLibrary.Conv_IntToDouble` (`self.Heat`)) 100.0)))

(fn `Modify Energy`
  (params (Amount :type Integer))
  (set `self.Energy` (`KismetMathLibrary.Clamp` (+ Amount (`self.Energy`)) 0 1000))
  (`self.Refresh Energy UI`)
  (return))

(fn `Modify Health`
  (params (Amount :type Integer))
  (set `self.Health` (`KismetMathLibrary.Clamp` (+ Amount (`self.Health`)) 0 100))
  (bind _newparam (`self.Get Health UI`))
  (set `self.HealthF` _newparam)
  (return))

(fn `Modify Heat`
  (params (Amount :type Integer))
  (set `self.Heat` (`KismetMathLibrary.Clamp` (+ Amount (`self.Heat`)) 0 100))
  (`self.Refresh Heat UI`)
  (return))

(fn `Refresh Energy UI`
  (bind _newparam (`self.Get Energy UI`))
  (set `self.EnergyF` _newparam)
  (return))

(fn `Refresh Heat UI`
  (bind _newparam (`self.Get Heat UI`))
  (set `self.HeatF` _newparam)
  (return))

(fn `Regenerate Health`
  (params (DeltaTime :type "Float (double-precision)"))
  (locals (HealthRegenerationPerSecond :type "Float (double-precision)" :default 0.5))
  (bind _health (`self.Health`))
  (bind _timebeforeregeneration (`self.TimeBeforeRegeneration`))
  (if (< _health 100)
    (`|ExecutionSequence`
      (:`then_0`
        (`/Engine/EditorBlueprintResources/StandardMacros.DoOnce` false :!label _label
          (:`Completed`
            (set `self.TempHealth` (`KismetMathLibrary.Conv_IntToDouble` _health)))))
      (:`then_1`
        (if (>= _health (`self.LastSavedHealth`))
          (`/Engine/EditorBlueprintResources/StandardMacros.CompareFloat` _timebeforeregeneration
            (:`>`
              (set `self.TimeBeforeRegeneration` (- _timebeforeregeneration DeltaTime)))
            (:`==`
              (bind _output_get (set `self.TempHealth` (+ (* DeltaTime (`local.HealthRegenerationPerSecond`)) (`self.TempHealth`)) :!label _label_2))
              (set `self.Health` (`KismetMathLibrary.Clamp` (`KismetMathLibrary.FFloor` _output_get) 0 100)))
            (:`<`
              (goto _label_2)))
          (else
            (`|ExecutionSequence`
              (:`then_0`
                (goto _label :!via `Reset`))
              (:`then_1`
                (set `self.TimeBeforeRegeneration` 3.0)))))
        (set `self.LastSavedHealth` _health)
        (return)))
    (else
      (return))))