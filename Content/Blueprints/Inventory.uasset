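; Player inventory of consumable flares and rations that restore the first-person character's heat and energy.
; Tick polls input: holding F while left-clicking uses a flare, and right-clicking uses a ration.
; InputGetKeyDown detects fresh presses by storing each button's previous state.
; Consume functions decrement positive counts, then modify the character's Vitality, though ConsumeRations is called without a character, so its cast stops before energy is restored.
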(event `self.ReceiveBeginPlay`
  (set `self.Player Controller` (`GameplayStatics.GetPlayerController` 0))
  (set `self.Character` (`GameplayStatics.GetPlayerCharacter` 0)))

(event `self.ReceiveTick`
  (params (DeltaSeconds :type "Float (single-precision)"))
  (bind _player_controller (`self.Player Controller`))
  ;[1 1 1] Consume Inventory
  (bind _output_get (set `self.InventoryOpened` (`PlayerController.IsInputKeyDown` _player_controller "F")))
  (bind _return (`self.Input Get Key Down` _player_controller "LeftMouseButton" true))
  (bind _return_2 (`self.Input Get Key Down` _player_controller "RightMouseButton"))
  (if (and _output_get _return)
    (`self.Consume Flares` (`self.Character`)))
  (if (and _output_get _return_2)
    (`self.Consume Rations` null)))

(fn `Consume Flares`
  (params (Player :type "Character Object Reference"))
  (bind _flares__ (`self.Flares #`))
  (`/Engine/EditorBlueprintResources/StandardMacros.CompareInt` _flares__
    (:`>`
      (`/Engine/EditorBlueprintResources/StandardMacros.DecrementInt` _flares__
        (:`  `
          (bind _asfirst_person_character (cast `/Game/FirstPersonBP/Blueprints/FirstPersonCharacter` Player))
          (`/Game/Blueprints/Vitality.Modify Heat` (`/Game/FirstPersonBP/Blueprints/FirstPersonCharacter.Vitality` _asfirst_person_character) (`self.Heat Rec per Flare`)))))
    (:`==`
      _)
    (:`<`
      _))
  (return))

(fn `Consume Rations`
  (params (NewParam :type "Character Object Reference"))
  (bind _rations__ (`self.Rations #`))
  (`/Engine/EditorBlueprintResources/StandardMacros.CompareInt` _rations__
    (:`>`
      (`/Engine/EditorBlueprintResources/StandardMacros.DecrementInt` _rations__
        (:`  `
          (bind _asfirst_person_character (cast `/Game/FirstPersonBP/Blueprints/FirstPersonCharacter` NewParam))
          (`/Game/Blueprints/Vitality.Modify Energy` (`/Game/FirstPersonBP/Blueprints/FirstPersonCharacter.Vitality` _asfirst_person_character) (`self.Energy Rec per Ration`)))))
    (:`==`
      _)
    (:`<`
      _))
  (return))

(fn `Input Get Key Down`
  (params (Character :type "PlayerController Object Reference") (Key :type "Key Structure" :default "AnyKey") (`Left/Right` :type Boolean))
  (returns (Return :type Boolean))
  (locals (`Return Val` :type Boolean))
  (bind _returnvalue (`PlayerController.IsInputKeyDown` Character Key))
  (bind _return_val (`local.Return Val`))
  (if `Left/Right`
    (set `local.Return Val` (and _returnvalue (not (`self.Clicked Left`))))
    (set `self.Clicked Left` _returnvalue)
    (return _return_val)
    (else
      (set `local.Return Val` (and (not (`self.Clicked Right`)) _returnvalue))
      (set `self.Clicked Right` _returnvalue)
      (return _return_val))))